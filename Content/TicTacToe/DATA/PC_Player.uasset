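; Player controller for a human player in a TicTacToe game, handling turn state, symbol and board reference through the IPlayerController interface.
; The cross symbol starts first; NextPlayerTurn ends the turn and passes it to the stored next player.
; The IsTurning OnRep toggles click events, with a short delay in TurnBegin as a workaround for click enabling when starting as nought.
; ShowWinner creates the winner widget for this player.
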(event EventNextPlayerTurn
  ;[1 0.8155 0] IPlayerController
  (bind _next_player (Variables|Default|GetNext%20Player)
    (:then
      (Class|IPlayerController|TurnEnd)
      (Class|IPlayerController|TurnBegin(Message) _next_player))
    (:else)))

(event EventSetBoardReference
  (params (boardRef :type A%20Board%20Object%20Reference))
  ;[1 0.8155 0] IPlayerController
  (Variables|Default|SetBoard%20Ref boardRef))

(event EventSetNextPlayerReference
  (params (l_NextPlayer :type Actor%20Object%20Reference))
  ;[1 0.8155 0] IPlayerController
  (Variables|Default|SetNext%20Player l_NextPlayer))

(event EventTurnBegin
  ;[1 0.8155 0] IPlayerController
  ;;[1 1 1] Когда игрок начинает за нолик, без Delay, не включается его EnableClickEvent
  (Utilities|FlowControl|Delay 0.2) ; костыль :)
  (Variables|Default|SetisTurning true))

(event EventTurnEnd
  ;[1 0.8155 0] IPlayerController
  (Variables|Default|SetisTurning false))

(event EventSetSymbol
  (params (l_Symbol :type PlayersSymbol%20Enum%20%28by%20ref%29 :default "PSymb_None"))
  ;[1 0.8155 0] IPlayerController
  (bind _output_get (Variables|Default|SetMySymbol l_Symbol))
  (Variables|Default|SetisTurning (Utilities|Enum|Equal(Enum) _output_get "PSymb_Cross")))

(event EventShowWinner
  (params (winnner :type PlayersSymbol%20Enum :default "PSymb_None"))
  ;[1 0.8155 0] IPlayerController
  (bind _returnvalue (UserInterface|CreateWidget "/Game/TicTacToe/UI/WBP_Winner.WBP_Winner_C" self))
  (UserInterface|Viewport|AddtoViewport _returnvalue 0)
  (Default|SetWinner _returnvalue winnner))

(fn ConstructionScript)

(fn OnRepIsTurning
  (Variables|Default|SetbEnableClickEvents (Variables|Default|GetisTurning)))

(fn GetIsTurningController
  (return (Variables|Default|GetisTurning)))

(fn GetSymbol
  (return (Variables|Default|GetMySymbol) true))